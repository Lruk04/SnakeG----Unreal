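; BP_SnakeGameMode is the game mode that sets up a two-player local snake game on BeginPlay.
; After a short delay, it creates a second local player and spawns two BP_SnakePawn actors at fixed, separate locations.
; Each player controller possesses one pawn and receives the same IMC_Player1 Enhanced Input mapping context, differing only in priority.
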(event `self.ReceiveBeginPlay`
  (bind _returnvalue (`GameplayStatics.GetPlayerController` 0))
  (bind _returnvalue_2 (`GameplayStatics.GetPlayerController` 1))
  (`KismetSystemLibrary.Delay` 1.0)
  (set `self.Spawn1` (50.0 50.0 92.0))
  (set `self.Spawn2` (350.0 350.0 92.0))
  (`GameplayStatics.CreatePlayer` 1)
  (bind _returnvalue_3 (`|SpawnActorFromClass` "/Game/Blueprints/Player/BP_SnakePawn.BP_SnakePawn_C" (`KismetMathLibrary.Conv_VectorToTransform` (`self.Spawn1`)) "Undefined" "MultiplyWithRoot" null null))
  (`Controller.Possess` _returnvalue_2 _returnvalue_3)
  (`EnhancedInputSubsystemInterface.AddMappingContext` (pcsubsystem `EnhancedInputLocalPlayerSubsystem` _returnvalue_2) "/Game/Input/IMC_Player1.IMC_Player1" 1 (struct))
  (bind _returnvalue_4 (`|SpawnActorFromClass` "/Game/Blueprints/Player/BP_SnakePawn.BP_SnakePawn_C" (`KismetMathLibrary.Conv_VectorToTransform` (`self.Spawn2`)) "Undefined" "MultiplyWithRoot" null null))
  (`Controller.Possess` _returnvalue _returnvalue_4)
  (`EnhancedInputSubsystemInterface.AddMappingContext` (pcsubsystem `EnhancedInputLocalPlayerSubsystem` _returnvalue) "/Game/Input/IMC_Player1.IMC_Player1" 0 (struct)))

(fn `UserConstructionScript`)