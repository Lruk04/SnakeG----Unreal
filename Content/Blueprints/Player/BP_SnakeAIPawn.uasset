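; BP_SnakeAIPawn is a snake AI pawn Blueprint that smoothly turns the snake's head toward its forward rotation.
; Every Tick calls UpdateHeadRotation, which blends the Head component's relative rotation toward ForwardRotation with a quaternion slerp scaled by delta time.
; The Blueprint contains no AI decision or movement logic and only reads ForwardRotation.
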(event `self.ReceiveTick`
  (params (DeltaSeconds :type "Float (single-precision)"))
  (`self.UpdateHeadRotation` DeltaSeconds))

(fn `UpdateHeadRotation`
  (params (DeltaTime :type "Float (double-precision)"))
  (`SceneComponent.K2_SetRelativeRotation` (`self.Head`) (`KismetMathLibrary.Quat_Rotator` (`KismetMathLibrary.Quat_Slerp` (`KismetMathLibrary.Conv_RotatorToQuaternion` (`SceneComponent.RelativeRotation` (`self.Head`))) (`KismetMathLibrary.Conv_RotatorToQuaternion` (`self.ForwardRotation`)) (* DeltaTime 20.0))) false false))

(fn `UserConstructionScript`)